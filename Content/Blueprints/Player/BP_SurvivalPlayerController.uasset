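; Player controller for a survival game that owns the player's UI: HUD, inventory, pause menu, map, loot menu, notifications, hit marker and death screen.
; Most widgets are created lazily and cached, while the loot menu is rebuilt on each show.
; Input opens pause, shows the map while held, and opens inventory in UI-only mode.
; C++ restart calls ShowinGameUI to rebuild the HUD and notification stack; death clears widgets before showing the killer screen.
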(event Custom|Open%20Pause%20Menu
  ;[0 0 0] Open/Close Pause Menu
  (Utilities|IsValid (Variables|Default|GetPauseWidget)
    (:Is%20Valid
      _)
    (:Is%20Not%20Valid
      (bind _returnvalue (UserInterface|CreateWidget "/Game/UserInterface/Widgets/Pause/WBP_PauseMenu.WBP_PauseMenu_C"))
      (Variables|Default|SetPauseWidget _returnvalue)))
  (UserInterface|Viewport|AddtoViewport (Variables|Default|GetPauseWidget) 0))

(event Custom|Close%20Pause%20Menu
  ;[0 0 0] Open/Close Pause Menu
  (Utilities|IsValid (Variables|Default|GetPauseWidget)
    (:Is%20Valid
      (Widget|RemovefromParent (Variables|Default|GetPauseWidget)))))

(event Custom|CreateNotificationUI
  ;[1 0 0.3226 1 15] Adds the Notification Widget to the screen. This doesn't means that is gonna show a notification, it just will place it.
  (Utilities|IsValid (Variables|Default|GetNotificationWidget)
    (:Is%20Valid
      _)
    (:Is%20Not%20Valid
      (bind _returnvalue (UserInterface|CreateWidget "/Game/UserInterface/Widgets/WBP_NotificationStack.WBP_NotificationStack_C"))
      (Variables|Default|SetNotificationWidget _returnvalue)))
  (UserInterface|Viewport|AddtoViewport (Variables|Default|GetNotificationWidget) 0))

(event Custom|Add%20InGame%20UI
  ;[0.3643 1 0.1127] Initial InGameUI. Called From C++, Survival Character, Restart Function.
  (Utilities|IsValid (Variables|Default|GetInGameWidget)
    (:Is%20Valid
      _)
    (:Is%20Not%20Valid
      (bind _returnvalue (UserInterface|CreateWidget "/Game/UserInterface/Widgets/WBP_Main.WBP_Main_C"))
      (Variables|Default|SetInGameWidget _returnvalue)))
  (UserInterface|Viewport|AddtoViewport (Variables|Default|GetInGameWidget) 0))

(event EventShowinGameUI
  ;[0.3643 1 0.1127] Initial InGameUI. Called From C++, Survival Character, Restart Function.
  (if (Pawn|IsLocalPlayerController)
    (Viewport|RemoveAllWidgets)
    (CallFunction|AddinGameUI)
    (CallFunction|CreateNotificationUI)))

(event EventShowNotification
  (params (Message :type Text%20%28by%20ref%29))
  (bind _notificationwidget (Variables|Default|GetNotificationWidget))
  ;[1 0.9733 0.05387] Spawns notification on screen
  (Utilities|IsValid _notificationwidget
    (:Is%20Valid
      (Default|AddNotification _notificationwidget Message))))

(event EventShowLootMenu
  (params (LootSource :type Inventory%20Component%20Object%20Reference))
  ;[0 1 0.9722] Show/Hide Loot Menu UI
  (bind _returnvalue (UserInterface|CreateWidget "/Game/UserInterface/Widgets/WBP_LootMenu.WBP_LootMenu_C"))
  (bind _output_get (Variables|Default|SetLootMenuWidget _returnvalue))
  (UserInterface|Viewport|AddtoViewport _output_get 0))

(event EventHideLootMenu
  ;[0 1 0.9722] Show/Hide Loot Menu UI
  (Widget|RemovefromParent (Variables|Default|GetLootMenuWidget)))

(event EventOnHitPlayer
  (bind _ingamewidget (Variables|Default|GetInGameWidget))
  ;[0 0 0] Show Hit Marker HUD
  (UserInterface|Animation|PlayAnimation _ingamewidget (Variables|/Game/UserInterface/Widgets/WBP_Main.WBP_Main_C|GetHitMarkerAnim _ingamewidget) 0.0 1 "Forward" 1.0 false))

(event EventBeginPlay
  ;[0 0.3366 1] Create Inventory Widget on Begin Play
  (if (Pawn|IsLocalPlayerController)
    (Utilities|IsValid (Variables|Default|GetInventoryWidget)
      (:Is%20Not%20Valid
        (bind _returnvalue (UserInterface|CreateWidget "/Game/UserInterface/Widgets/WBP_Inventory.WBP_Inventory_C"))
        (Variables|Default|SetInventoryWidget _returnvalue)
        (Input|SetInputModeGameOnly self)
        (Variables|Default|SetbShowMouseCursor false)))))

(event EventShowDeathScreen
  (params (Killer :type Survival%20Character%20Object%20Reference))
  ;[0.6094 0 0] Death Screen
  (Viewport|RemoveAllWidgets)
  (bind _asbp_survival_character (Utilities|Casting|CastToBP_SurvivalCharacter Killer))
  (Variables|Default|GetDeathScreenWidget
    (:then
      _)
    (:else
      (bind _returnvalue (UserInterface|CreateWidget "/Game/UserInterface/Widgets/WBP_DeathScreen.WBP_DeathScreen_C" 0 _asbp_survival_character))
      (Variables|Default|SetDeathScreenWidget _returnvalue)))
  (UserInterface|Viewport|AddtoViewport (Variables|Default|GetDeathScreenWidget) 0))

(event Input|ActionEvents|InputActionOpenInventory
  (params (Key :type Key%20Structure :default "None"))
  ;[1 0 0] Open Player Inventory
  (:Pressed
    (Utilities|IsValid (Variables|Default|GetInventoryWidget)
      (:Is%20Valid
        _)
      (:Is%20Not%20Valid
        (bind _returnvalue (UserInterface|CreateWidget "/Game/UserInterface/Widgets/WBP_Inventory.WBP_Inventory_C"))
        (Variables|Default|SetInventoryWidget _returnvalue)))
    (UserInterface|Viewport|AddtoViewport (Variables|Default|GetInventoryWidget) 0)
    (Variables|Default|SetbShowMouseCursor true)
    (Input|SetInputModeUIOnly self (Variables|Default|GetInventoryWidget) "DoNotLock")))

(event Input|ActionEvents|InputActionOpenMap
  (params (Key :type Key%20Structure :default "None"))
  ;[1 0.8233 0] Open Map
  (:Pressed
    (Utilities|IsValid (Variables|Default|GetMapWidget)
      (:Is%20Valid
        _)
      (:Is%20Not%20Valid
        (bind _returnvalue (UserInterface|CreateWidget "/Game/UserInterface/Widgets/WBP_Map.WBP_Map_C"))
        (Variables|Default|SetMapWidget _returnvalue)))
    (UserInterface|Viewport|AddtoViewport (Variables|Default|GetMapWidget) 0))
  (:Released
    (Widget|RemovefromParent (Variables|Default|GetMapWidget))))

(event Input|ActionEvents|InputActionOpenPauseMenu
  (params (Key :type Key%20Structure :default "None"))
  ;[0 0 0] Open/Close Pause Menu
  (:Pressed
    (CallFunction|OpenPauseMenu)))

(fn ConstructionScript)