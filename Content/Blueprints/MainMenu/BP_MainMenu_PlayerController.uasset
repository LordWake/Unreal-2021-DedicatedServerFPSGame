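; Player controller for the main menu that puts the main menu widget on screen.
; On BeginPlay, only the local player controller calls ShowMainMenu.
; ShowMainMenu creates WBP_MainMenu owned by the controller if no valid instance exists, caches it in MenuWidget and adds it to the viewport.
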(event Custom|Show%20Main%20Menu
  (Utilities|IsValid (Variables|Default|GetMenuWidget)
    (:Is%20Valid
      _)
    (:Is%20Not%20Valid
      (bind _returnvalue (UserInterface|CreateWidget "/Game/UserInterface/Widgets/MainMenu/WBP_MainMenu.WBP_MainMenu_C" self))
      (Variables|Default|SetMenuWidget _returnvalue)))
  (UserInterface|Viewport|AddtoViewport (Variables|Default|GetMenuWidget) 0))

(event EventBeginPlay
  (if (Pawn|IsLocalPlayerController)
    (CallFunction|ShowMainMenu)))

(fn ConstructionScript)