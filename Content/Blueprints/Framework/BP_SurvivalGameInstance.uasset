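; Game instance for the survival game that handles joining online sessions and leaving the game.
; TryJoinGame searches sessions filtered on a Spacewar GAMENAME property and passes the first result to JoinSession, which switches to game-only input and hides the cursor.
; Search or join failures report through CallOnFailedToFindMatch.
; Both quit events destroy the session, then exit to desktop or open MainMenu whether destruction succeeds or fails.
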(event Custom|Try%20Join%20Game
  (bind _results (|FindSessionsAdvanced (Game|GetPlayerController 0) 1000 false "AllServers" (Utilities|Array|MakeArray (Class|AdvancedSessionsLibrary|MakeLiteralSessionSearchProperty (Class|AdvancedSessionsLibrary|MakeLiteralSessionPropertyString "GAMENAME" "Spacewar") "Equals")) false false false)
    (:OnSuccess
      (CallFunction|JoinSession (Utilities|Array|Get(acopy) _results)))
    (:OnFailure
      (Default|CallOnFailedtoFindMatch "Find Sessions Failed"))))

(event Custom|Join%20Session
  (params (Session :type Blueprint%20Session%20Result%20Structure))
  (bind _returnvalue (Game|GetPlayerController 0))
  (|JoinSession (Game|GetPlayerController 0) Session
    (:then
      (Input|SetInputModeGameOnly _returnvalue :!label _label)
      (Variables|/Script/Engine.PlayerController|SetbShowMouseCursor _returnvalue false))
    (:OnSuccess
      (goto _label))
    (:OnFailure
      (Default|CallOnFailedtoFindMatch "Failed to join session"))))

(event Custom|OnQuitToDesktop
  (|DestroySession (Game|GetPlayerController 0)
    (:OnSuccess
      _)
    (:OnFailure
      _))
  (Game|QuitGame 0 "Quit" false))

(event Custom|OnQuitToMenu
  (|DestroySession (Game|GetPlayerController 0)
    (:OnSuccess
      _)
    (:OnFailure
      _))
  (Game|OpenLevel(byName) "MainMenu"))