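; BP_SUV is a drivable, networked SUV that players enter through an Interaction component and drive with throttle, steering, handbrake and look input.
; On interact, the authority waits briefly, possesses the SUV, records the Driver and hides the character.
; Exit works only below a speed threshold, restoring the character at ExitLocation and repossessing it.
; Driver's RepNotify toggles interaction, pawn collision and physics simulation according to occupancy.
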(event OnInteract(Interaction)
  (params (Character :type Survival%20Character%20Object%20Reference))
  (bind _returnvalue (Pawn|GetController Character))
  ;[0 0.9043 1] Get into Vehicle
  (Networking|SwitchHasAuthority
    (:Authority
      (Utilities|FlowControl|Delay 0.5)
      (Pawn|Possess _returnvalue self)
      (Actor|SetOwner _returnvalue)
      (Variables|Default|SetDriver Character)
      (Rendering|SetActorHiddenInGame Character true))
    (:Remote
      (Rendering|SetVisibility (Variables|Default|GetInteraction) false false))))

(event Custom|Exit%20Vehicle
  ;[1 0.3333 0] Exit Vehicle
  (CallFunction|ServerExitVehicle))

(event Custom|Server%20Exit%20Vehicle
  ;[1 0.3333 0] Exit Vehicle
  (Rendering|SetActorHiddenInGame (Variables|Default|GetDriver) false)
  (Transformation|SetActorLocation (Variables|Default|GetDriver) (Transformation|GetWorldLocation (Variables|Default|GetExitLocation)) false true)
  (Pawn|Possess (Pawn|GetController) (Variables|Default|GetDriver))
  (Actor|SetOwner 0)
  (Variables|Default|SetDriver 0))

(event Input|ActionEvents|InputActionInteract
  (params (Key :type Key%20Structure))
  ;[1 0.3333 0] Exit Vehicle
  (:Pressed
    (if (<= (Class|WheeledVehicleMovementComponent|GetForwardSpeed (Variables|Default|GetVehicleMovement)) 5e+01)
      (CallFunction|ExitVehicle))))

(event Input|ActionEvents|InputActionHandBrake
  (params (Key :type Key%20Structure))
  (bind _vehiclemovement (Variables|Default|GetVehicleMovement))
  ;[0.2273 1 0] Movement
  (:Pressed
    (Class|WheeledVehicleMovementComponent|SetHandbrakeInput _vehiclemovement true))
  (:Released
    (Class|WheeledVehicleMovementComponent|SetHandbrakeInput _vehiclemovement false)))

(event Input|AxisEvents|InputAxisMoveForward
  (params (AxisValue :type Float%20%28single-precision%29))
  ;[0.2273 1 0] Movement
  (Class|WheeledVehicleMovementComponent|SetThrottleInput (Variables|Default|GetVehicleMovement) AxisValue))

(event Input|AxisEvents|InputAxisMoveRight
  (params (AxisValue :type Float%20%28single-precision%29))
  ;[0.2273 1 0] Movement
  (Class|WheeledVehicleMovementComponent|SetSteeringInput (Variables|Default|GetVehicleMovement) AxisValue))

(event Input|AxisEvents|InputAxisLookUp
  (params (AxisValue :type Float%20%28single-precision%29))
  ;[0.2273 1 0] Movement
  (Pawn|Input|AddControllerPitchInput (* AxisValue -1.0)))

(event Input|AxisEvents|InputAxisTurn
  (params (AxisValue :type Float%20%28single-precision%29))
  ;[0.2273 1 0] Movement
  (Pawn|Input|AddControllerYawInput AxisValue))

(fn ConstructionScript)

(fn OnRepDriver
  (bind _returnvalue (Pawn|GetController))
  (bind _interaction (Variables|Default|GetInteraction))
  (bind _mesh (Variables|Character|GetMesh))
  (bind _mesh_2 (Variables|Character|GetMesh))
  (Utilities|IsValid (Variables|Default|GetDriver)
    (:Is%20Valid
      (Components|Activation|Deactivate _interaction)
      (Rendering|SetRenderCustomDepth _mesh false)
      (Collision|SetCollisionResponsetoChannel _mesh "ECC_Pawn" "ECR_Overlap")
      (Physics|SetSimulatePhysics _mesh_2 true)
      (Utilities|IsValid _returnvalue
        (:Is%20Valid
          (Pawn|SetControlRotation _returnvalue (Transformation|GetActorRotation)))))
    (:Is%20Not%20Valid
      (Components|Activation|Activate _interaction true)
      (Collision|SetCollisionResponsetoChannel _mesh "ECC_Pawn" "ECR_Block")
      (Physics|SetSimulatePhysics _mesh_2 false))))